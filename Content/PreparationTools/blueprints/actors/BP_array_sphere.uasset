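; Preview actor that lays out a centered, near-square grid of static meshes, one per material in ArrayMat.
; The construction script first rebuilds ArrayMat with unique entries up to MaxMat, ignoring an empty last slot.
; Grid dimensions come from the square root of the count, and a partial last row is centered.
; Meshes attach to an offset Billboard at Distancing intervals, with Invert reversing material order.
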(fn ConstructionScript
  (bind _output_get (LocalVariables|SetTmpArrayMat (Variables|Default|GetArrayMat))) ; prevent losing items
  (CallFunction|CompactArray _output_get (Variables|Default|GetArrayMat) (Variables|Default|GetMaxMat))
  (bind _output_get_2 (LocalVariables|SetTrueLength (Math|Integer|SelectInt (Utilities|Array|Length (Variables|Default|GetArrayMat)) (- (Utilities|Array|Length (Variables|Default|GetArrayMat)) 1) (Utilities|IsValid (Utilities|Array|Get(acopy) (Variables|Default|GetArrayMat) (Utilities|Array|LastIndex (Variables|Default|GetArrayMat)))))))
  (LocalVariables|SetTrueLastIndex (- _output_get_2 1)) ; length of valid items
  (bind _output_get_3 (LocalVariables|SetSQRT-1 (Math|Float|Clamp(Float) (- (Math|Float|Sqrt (Math|Conversions|ToFloat(Integer) (LocalVariables|GetTrueLength))) 1.0) 0.0 (Math|Conversions|ToFloat(Integer) (Variables|Default|GetMaxMat)))))
  (bind _output_get_4 (LocalVariables|SetLastX (Math|Float|Ceil _output_get_3)))
  (LocalVariables|SetMaxItemX (+ _output_get_4 1))
  (LocalVariables|SetLastY (Math|Float|Round (LocalVariables|GetSQRT-1)))
  (Transformation|AddLocalOffset (Variables|Default|GetBillboard) (Math|Vector|MakeVector (Utilities|/2*(-1) (Utilities|CalLoc (LocalVariables|GetLastX))) (Utilities|/2*(-1) (Utilities|CalLoc (LocalVariables|GetLastY))) 0.0) false false) ; center the array
  (LocalVariables|SetDeltaX (- (* (LocalVariables|GetMaxItemX) (+ (LocalVariables|GetLastY) 1)) (LocalVariables|GetTrueLength)))
  (LocalVariables|SetOffsetLastY (/ (Utilities|CalLoc (LocalVariables|GetDeltaX)) 2.0))
  (for _index (range 0 (LocalVariables|GetLastY)) ; Y
    (LocalVariables|SetLocY (Utilities|CalLoc _index))
    (LocalVariables|SetIsLastY (== (LocalVariables|GetLastY) _index))
    (LocalVariables|SetTrueLastX (Math|Integer|SelectInt (- (LocalVariables|GetLastX) (LocalVariables|GetDeltaX)) (LocalVariables|GetLastX) (LocalVariables|GetIsLastY)))
    (LocalVariables|SetSumItemsLastY (* (LocalVariables|GetMaxItemX) _index))
    (for _index_2 (range 0 (LocalVariables|GetTrueLastX)) ; X
      (bind _returnvalue (AddComponent|AddStaticMeshComponent false (Math|Transform|MakeTransform (Math|Vector|MakeVector (Math|Float|SelectFloat (+ (LocalVariables|GetOffsetLastY) (Utilities|CalLoc _index_2)) (Utilities|CalLoc _index_2) (LocalVariables|GetIsLastY)) (LocalVariables|GetLocY) 0.0) "0, 0, 0" "1,1,1")))
      (Rendering|Material|SetMaterial _returnvalue 0 (Utilities|Array|Get(acopy) (Variables|Default|GetArrayMat) (Math|Integer|SelectInt (- (LocalVariables|GetTrueLastIndex) (+ (LocalVariables|GetSumItemsLastY) _index_2)) (+ (LocalVariables|GetSumItemsLastY) _index_2) (Variables|Default|Getinvert))))
      (Transformation|AttachComponentToComponent _returnvalue (Variables|Default|GetBillboard) "None" "KeepRelative" "KeepRelative" "KeepRelative" false))))

(fn CompactArray
  (params (TmpArray :type Array%20of%20Object%20Object%20References) (TargetArray :type Array%20of%20Object%20Object%20References) (max :type Integer%20%28by%20ref%29))
  (Utilities|Array|Clear TargetArray)
  (for _index (range 0 (- max 1))
    (Utilities|Array|AddUnique TargetArray (Utilities|Array|Get(acopy) TmpArray _index)))
  (return))