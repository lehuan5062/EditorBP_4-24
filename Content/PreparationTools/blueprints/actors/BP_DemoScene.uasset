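; BP_DemoScene is a demo scene actor that bundles a directional sun light, a sky light and a cube.
; Its construction script applies sun specular scale and rotation, cube location and scale, and a vertical sky light offset from variables, then recaptures the sky.
; A separate capture event triggers the sky light recapture on demand.
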(event Custom|capture
  (Class|SkyLightComponent|RecaptureSky (Variables|Default|GetSkyLight)))

(fn ConstructionScript
  (Class|LightComponent|SetSpecularScale (Variables|Default|GetDirectionalLight) (Variables|Default|GetSunSpecular))
  (Transformation|SetWorldRotation (Variables|Default|GetDirectionalLight) (Variables|Default|GetRotSun) false false)
  (Transformation|SetRelativeTransform (Variables|Default|GetCube) (Math|Transform|MakeTransform (Variables|Default|GetLocCube) "0, 0, 0" (Variables|Default|GetScaleCube)) false false)
  (Transformation|AddLocalOffset (Variables|Default|GetSkyLight) (Math|Vector|MakeVector 0.0 0.0 (Variables|Default|GetSkyLightHeight)) false false)
  (Class|SkyLightComponent|RecaptureSky (Variables|Default|GetSkyLight)))