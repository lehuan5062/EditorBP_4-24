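; Preparation tool actor whose construction script lays out manually assigned static meshes in a centered X-by-Y grid, repeating each mesh per material variation.
; It de-duplicates and resizes the mesh and material arrays, then spawns components under an offset Billboard, pairing materials by index.
; A partially filled last row gets re-centered, and Invert reverses the assignment order.
; A name-based material mapping branch is left disconnected.
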(fn ConstructionScript
  (LocalVariables|SetLastIndexSM (- (Variables|Default|GetMaxSM) 1))
  (bind _output_get (LocalVariables|SetTmpArraySM (Variables|Default|GetArray_SM))) ; prevent losing items
  (Utilities|CompactArray _output_get (Variables|Default|GetArray_SM) (LocalVariables|GetLastIndexSM))
  (bind _output_get_2 (LocalVariables|SetTrueLength (Math|Integer|SelectInt (Utilities|Array|Length (Variables|Default|GetArray_SM)) (- (Utilities|Array|Length (Variables|Default|GetArray_SM)) 1) (Utilities|IsValid (Utilities|Array|Get(acopy) (Variables|Default|GetArray_SM) (Utilities|Array|LastIndex (Variables|Default|GetArray_SM))))))) ; length of valid items
  (LocalVariables|SetTrueLastIndex (- _output_get_2 1))
  (LocalVariables|SetLastIndexX (- (Variables|Default|Getx) 1))
  (LocalVariables|SetLastIndexY (- (Variables|Default|Gety) 1))
  (LocalVariables|SetLastVariant (- (Variables|Default|Getvariations) 1))
  (Transformation|AddLocalOffset (Variables|Default|GetBillboard) (Math|Vector|MakeVector (CallFunction|/2*(-1) (CallFunction|DistanceVariant+DistanceX (* (Variables|Default|Getx) (LocalVariables|GetLastVariant)) (LocalVariables|GetLastIndexX))) (CallFunction|/2*(-1) (CallFunction|CalLocY (LocalVariables|GetLastIndexY))) 0.0) false false) ; center the array
  (bind _output_get_3 (LocalVariables|SetDeltaX (- (* (Variables|Default|Getx) (Variables|Default|Gety)) (LocalVariables|GetTrueLength))))
  (LocalVariables|SetOffsetLastIndexY (/ (CallFunction|DistanceVariant+DistanceX (* _output_get_3 (LocalVariables|GetLastVariant)) (LocalVariables|GetDeltaX)) 2.0))
  (LocalVariables|SetLastIndexMat (- (* (Variables|Default|GetMaxSM) (Variables|Default|Getvariations)) 1))
  (bind _output_get_4 (LocalVariables|SetTmpArrayMat (Variables|Default|GetArrayMat))) ; prevent losing items
  (Utilities|CompactArray _output_get_4 (Variables|Default|GetArrayMat) (LocalVariables|GetLastIndexMat))
  (for _index (range 0 (LocalVariables|GetLastIndexY)) ; Y
    (LocalVariables|SetLocY (CallFunction|CalLocY _index))
    (LocalVariables|SetIsLastIndexY (== (LocalVariables|GetLastIndexY) _index))
    (LocalVariables|SetTrueLastIndexX (Math|Integer|SelectInt (- (LocalVariables|GetLastIndexX) (LocalVariables|GetDeltaX)) (LocalVariables|GetLastIndexX) (LocalVariables|GetIsLastIndexY)))
    (LocalVariables|SetSumItemsLastIndexY (* (Variables|Default|Getx) _index))
    (for _index_2 (range 0 (LocalVariables|GetTrueLastIndexX)) ; X
      (LocalVariables|SetDistanceVariantMultiplier (* (LocalVariables|GetLastVariant) _index_2))
      (LocalVariables|SetLocX (CallFunction|CalLocX _index_2))
      (bind _output_get_5 (LocalVariables|SetSumItems (+ (LocalVariables|GetSumItemsLastIndexY) _index_2)))
      (LocalVariables|SetFirstIndexMat (* _output_get_5 (Variables|Default|Getvariations)))
      (LocalVariables|SetCurrentSM (Utilities|Array|Get(acopy) (Variables|Default|GetArray_SM) (Math|Integer|SelectInt (- (LocalVariables|GetTrueLastIndex) (LocalVariables|GetSumItems)) (LocalVariables|GetSumItems) (Variables|Default|Getinvert))))
      (for _index_3 (range 0 (LocalVariables|GetLastVariant)) ; variations
        (bind _returnvalue (AddComponent|AddStaticMeshComponent false (Math|Transform|MakeTransform (Math|Vector|MakeVector (Math|Float|SelectFloat (+ (LocalVariables|GetOffsetLastIndexY) (+ (CallFunction|CalLocXVariant (+ (LocalVariables|GetDistanceVariantMultiplier) _index_3)) (LocalVariables|GetLocX))) (+ (CallFunction|CalLocXVariant (+ (LocalVariables|GetDistanceVariantMultiplier) _index_3)) (LocalVariables|GetLocX)) (LocalVariables|GetIsLastIndexY)) (LocalVariables|GetLocY) 0.0) (Variables|Default|Getrotation) "1,1,1")))
        (Rendering|Material|SetMaterial _returnvalue 0 (Utilities|Array|Get(acopy) (Variables|Default|GetArrayMat) (Math|Integer|SelectInt (- (LocalVariables|GetLastIndexMat) (+ _index_3 (LocalVariables|GetFirstIndexMat))) (+ _index_3 (LocalVariables|GetFirstIndexMat)) (Variables|Default|Getinvert))))
        (Components|StaticMesh|SetStaticMesh _returnvalue (LocalVariables|GetCurrentSM))
        (Transformation|AttachComponentToComponent _returnvalue (Variables|Default|GetBillboard) "None" "KeepRelative" "KeepRelative" "KeepRelative" false)))))

(fn DistanceVariant+DistanceX
  (params (X_variant :type Integer%20%28by%20ref%29) (X :type Integer%20%28by%20ref%29))
  (return (+ (CallFunction|CalLocXVariant X_variant) (CallFunction|CalLocX X))))

(fn CalLocXVariant
  (params (A :type Integer%20%28by%20ref%29))
  (return (* A (Variables|Default|GetDistanceVariant))))

(fn CalLocX
  (params (x :type Integer%20%28by%20ref%29))
  (return (* x (Variables|Default|GetDistanceX))))

(fn CalLocY
  (params (y :type Integer%20%28by%20ref%29))
  (return (* y (Variables|Default|GetDistanceY))))

(fn /2*(-1)
  (params (A :type Float%20%28single-precision%29%20%28by%20ref%29))
  (return (* -1 (/ A 2.0))))