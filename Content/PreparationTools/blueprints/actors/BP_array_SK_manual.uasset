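; Preparation-tool actor that lays out an array of skeletal meshes in a centered X by Y grid at construction, with several material variations of each mesh side by side.
; It compacts the mesh and material arrays to unique entries, offsets a partial last row to center it, and can invert the order.
; Materials are keyed by name with the first three characters chopped, then matched to mesh name plus a _1 to _4 suffix.
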(fn ConstructionScript
  (bind _output_get (LocalVariables|SetTmpArraySK (Variables|Default|GetArraySK)))
  (CallFunction|CompactArray _output_get (Variables|Default|GetArraySK) (Variables|Default|GetMaxSK))
  (bind _output_get_2 (LocalVariables|SetTrueLength (Math|Integer|SelectInt (Utilities|Array|Length (Variables|Default|GetArraySK)) (- (Utilities|Array|Length (Variables|Default|GetArraySK)) 1) (Utilities|IsValid (Utilities|Array|Get(acopy) (Variables|Default|GetArraySK) (Utilities|Array|LastIndex (Variables|Default|GetArraySK))))))) ; length of valid items
  (LocalVariables|SetTrueLastIndex (- _output_get_2 1))
  (LocalVariables|SetLastIndexX (- (Variables|Default|Getx) 1))
  (LocalVariables|SetLastIndexY (- (Variables|Default|Gety) 1))
  (LocalVariables|SetLastVariant (- (Variables|Default|Getvariations) 1))
  (Transformation|AddLocalOffset (Variables|Default|GetBillboard) (Math|Vector|MakeVector (Utilities|/2*(-1) (Utilities|DistanceX+DistanceVariant (* (Variables|Default|Getx) (LocalVariables|GetLastVariant)) (LocalVariables|GetLastIndexX))) (Utilities|/2*(-1) (Utilities|CalLocY (LocalVariables|GetLastIndexY))) 0.0) false false) ; center the array
  (bind _output_get_3 (LocalVariables|SetDeltaX (- (* (Variables|Default|Getx) (Variables|Default|Gety)) (LocalVariables|GetTrueLength))))
  (LocalVariables|SetOffsetLastIndexY (/ (Utilities|DistanceX+DistanceVariant (* _output_get_3 (LocalVariables|GetLastVariant)) (LocalVariables|GetDeltaX)) 2.0))
  (LocalVariables|SetMaxMat (* (Variables|Default|GetMaxSK) (Variables|Default|Getvariations)))
  (bind _output_get_4 (LocalVariables|SetTmpArrayMat (Variables|Default|GetArrayMat))) ; prevent losing items
  (CallFunction|CompactArray _output_get_4 (Variables|Default|GetArrayMat) (LocalVariables|GetMaxMat))
  (Utilities|Map|Clear (LocalVariables|GetMapMat))
  (for _array_element (Variables|Default|GetArrayMat)
    (Utilities|Map|Add (LocalVariables|GetMapMat) (Utilities|String|RightChop (Utilities|GetDisplayName _array_element) 3) _array_element) ; set keys based on naming
  )
  (for _index (range 0 (LocalVariables|GetLastIndexY)) ; Y
    (LocalVariables|SetLocY (Utilities|CalLocY _index))
    (LocalVariables|SetIsLastIndexY (== (LocalVariables|GetLastIndexY) _index))
    (LocalVariables|SetTrueLastIndexX (Math|Integer|SelectInt (- (LocalVariables|GetLastIndexX) (LocalVariables|GetDeltaX)) (LocalVariables|GetLastIndexX) (LocalVariables|GetIsLastIndexY)))
    (LocalVariables|SetSumItemsLastIndexY (* (Variables|Default|Getx) _index))
    (for _index_2 (range 0 (LocalVariables|GetTrueLastIndexX)) ; X
      (LocalVariables|SetDistanceVariantMultiplier (* (LocalVariables|GetLastVariant) _index_2))
      (LocalVariables|SetLocX (Utilities|CalLocX _index_2))
      (LocalVariables|SetCurrentSK (Utilities|Array|Get(acopy) (Variables|Default|GetArraySK) (Math|Integer|SelectInt (- (LocalVariables|GetTrueLastIndex) (+ (LocalVariables|GetSumItemsLastIndexY) _index_2)) (+ (LocalVariables|GetSumItemsLastIndexY) _index_2) (Variables|Default|Getinvert))))
      (for _index_3 (range 0 (LocalVariables|GetLastVariant)) ; variations
        (bind _returnvalue (AddComponent|AddSkeletalMeshComponent false (Math|Transform|MakeTransform (Math|Vector|MakeVector (Math|Float|SelectFloat (+ (LocalVariables|GetOffsetLastIndexY) (+ (Utilities|CalLocXVariant (+ (LocalVariables|GetDistanceVariantMultiplier) _index_3)) (LocalVariables|GetLocX))) (+ (Utilities|CalLocXVariant (+ (LocalVariables|GetDistanceVariantMultiplier) _index_3)) (LocalVariables|GetLocX)) (LocalVariables|GetIsLastIndexY)) (LocalVariables|GetLocY) 0.0) (Variables|Default|Getrotation) "1,1,1")))
        (Rendering|Material|SetMaterial _returnvalue 0 (.Value (Utilities|Map|Find (LocalVariables|GetMapMat) (Utilities|String|Append (Utilities|String|RightChop (Utilities|GetDisplayName (LocalVariables|GetCurrentSK)) 3) (Utilities|Select :Index (Math|Integer|SelectInt (- (LocalVariables|GetLastVariant) _index_3) _index_3 (Variables|Default|Getinvert)) :Option%200 "_1" :Option%201 "_2" :Option%202 "_3" :Option%203 "_4")))))
        (Class|SkinnedMeshComponent|SetSkeletalMesh _returnvalue (LocalVariables|GetCurrentSK) true)
        (Transformation|AttachComponentToComponent _returnvalue (Variables|Default|GetBillboard) "None" "KeepRelative" "KeepRelative" "KeepRelative" false)))))

(fn CompactArray
  (params (TmpArray :type Array%20of%20Object%20Object%20References) (TargetArray :type Array%20of%20Object%20Object%20References) (max :type Integer%20%28by%20ref%29))
  (Utilities|Array|Clear TargetArray)
  (for _index (range 0 (- max 1))
    (Utilities|Array|AddUnique TargetArray (Utilities|Array|Get(acopy) TmpArray _index)))
  (return))