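; Editor preparation actor that auto-lays out an array of static meshes in a centered, near-square grid, with material variations side by side.
; The construction script compacts the mesh and material arrays to unique entries, then derives grid size from the square root of the mesh count.
; It spawns mesh components under a Billboard, centering any partial last row and optionally inverting order.
; Materials are matched by naming convention: prefix-stripped mesh name plus a numbered suffix.
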(fn ConstructionScript
  (bind _output_get (LocalVariables|SetTmpArraySM (Variables|Default|GetArray_SM))) ; prevent losing items
  (CallFunction|CompactArray _output_get (Variables|Default|GetArray_SM) (Variables|Default|GetMaxSM))
  (bind _output_get_2 (LocalVariables|SetTrueLength (Math|Integer|SelectInt (Utilities|Array|Length (Variables|Default|GetArray_SM)) (- (Utilities|Array|Length (Variables|Default|GetArray_SM)) 1) (Utilities|IsValid (Utilities|Array|Get(acopy) (Variables|Default|GetArray_SM) (Utilities|Array|LastIndex (Variables|Default|GetArray_SM)))))))
  (LocalVariables|SetTrueLastIndex (- _output_get_2 1)) ; length of valid items
  (bind _output_get_3 (LocalVariables|SetSQRT-1 (Math|Float|Clamp(Float) (- (Math|Float|Sqrt (Math|Conversions|ToFloat(Integer) (LocalVariables|GetTrueLength))) 1.0) 0.0 (Math|Conversions|ToFloat(Integer) (Variables|Default|GetMaxSM)))))
  (bind _output_get_4 (LocalVariables|SetLastX (Math|Float|Ceil _output_get_3)))
  (LocalVariables|SetMaxItemX (+ _output_get_4 1))
  (LocalVariables|SetLastY (Math|Float|Round (LocalVariables|GetSQRT-1)))
  (LocalVariables|SetLastVariant (- (Variables|Default|Getvariations) 1))
  (Transformation|AddLocalOffset (Variables|Default|GetBillboard) (Math|Vector|MakeVector (Utilities|/2*(-1) (Utilities|DistanceX+DistanceVariant (* (LocalVariables|GetMaxItemX) (LocalVariables|GetLastVariant)) (LocalVariables|GetLastX))) (Utilities|/2*(-1) (Utilities|CalLocY (LocalVariables|GetLastY))) 0.0) false false) ; center the array
  (LocalVariables|SetDeltaX (- (* (LocalVariables|GetMaxItemX) (+ (LocalVariables|GetLastY) 1)) (LocalVariables|GetTrueLength)))
  (LocalVariables|SetOffsetLastY (/ (Utilities|DistanceX+DistanceVariant (* (LocalVariables|GetDeltaX) (LocalVariables|GetLastVariant)) (LocalVariables|GetDeltaX)) 2.0))
  (LocalVariables|SetMaxMat (* (Variables|Default|GetMaxSM) (Variables|Default|Getvariations)))
  (bind _output_get_5 (LocalVariables|SetTmpArrayMat (Variables|Default|GetArrayMat))) ; prevent losing items
  (CallFunction|CompactArray _output_get_5 (Variables|Default|GetArrayMat) (LocalVariables|GetMaxMat))
  (Utilities|Map|Clear (LocalVariables|GetMapMat))
  (for _array_element (Variables|Default|GetArrayMat)
    (Utilities|Map|Add (LocalVariables|GetMapMat) (Utilities|String|RightChop (Utilities|GetDisplayName _array_element) 3) _array_element) ; set keys based on naming
  )
  (for _index (range 0 (LocalVariables|GetLastY)) ; Y
    (LocalVariables|SetLocY (Utilities|CalLocY _index))
    (LocalVariables|SetIsLastY (== (LocalVariables|GetLastY) _index))
    (LocalVariables|SetTrueLastX (Math|Integer|SelectInt (- (LocalVariables|GetLastX) (LocalVariables|GetDeltaX)) (LocalVariables|GetLastX) (LocalVariables|GetIsLastY)))
    (LocalVariables|SetSumItemsLastY (* (LocalVariables|GetMaxItemX) _index))
    (for _index_2 (range 0 (LocalVariables|GetTrueLastX)) ; X
      (LocalVariables|SetDistanceVariantMultiplier (* (LocalVariables|GetLastVariant) _index_2))
      (LocalVariables|SetLocX (Utilities|CalLocX _index_2))
      (LocalVariables|SetCurrentSM (Utilities|Array|Get(acopy) (Variables|Default|GetArray_SM) (Math|Integer|SelectInt (- (LocalVariables|GetTrueLastIndex) (+ (LocalVariables|GetSumItemsLastY) _index_2)) (+ (LocalVariables|GetSumItemsLastY) _index_2) (Variables|Default|Getinvert))))
      (for _index_3 (range 0 (LocalVariables|GetLastVariant)) ; variations
        (bind _returnvalue (AddComponent|AddStaticMeshComponent false (Math|Transform|MakeTransform (Math|Vector|MakeVector (Math|Float|SelectFloat (+ (LocalVariables|GetOffsetLastY) (+ (Utilities|CalLocXVariant (+ (LocalVariables|GetDistanceVariantMultiplier) _index_3)) (LocalVariables|GetLocX))) (+ (Utilities|CalLocXVariant (+ (LocalVariables|GetDistanceVariantMultiplier) _index_3)) (LocalVariables|GetLocX)) (LocalVariables|GetIsLastY)) (LocalVariables|GetLocY) 0.0) (Variables|Default|Getrotation) "1,1,1")))
        (Rendering|Material|SetMaterial _returnvalue 0 (.Value (Utilities|Map|Find (LocalVariables|GetMapMat) (Utilities|String|Append (Utilities|String|Left (Utilities|String|RightChop (Utilities|GetDisplayName (LocalVariables|GetCurrentSM)) 3) 8) (Utilities|Select :Index (Math|Integer|SelectInt (- (LocalVariables|GetLastVariant) _index_3) _index_3 (Variables|Default|Getinvert)) :Option%200 "_1" :Option%201 "_2" :Option%202 "_3")))))
        (Components|StaticMesh|SetStaticMesh _returnvalue (LocalVariables|GetCurrentSM))
        (Transformation|AttachComponentToComponent _returnvalue (Variables|Default|GetBillboard) "None" "KeepRelative" "KeepRelative" "KeepRelative" false)))))

(fn CompactArray
  (params (TmpArray :type Array%20of%20Object%20Object%20References) (TargetArray :type Array%20of%20Object%20Object%20References) (max :type Integer%20%28by%20ref%29))
  (Utilities|Array|Clear TargetArray)
  (for _index (range 0 (- max 1))
    (Utilities|Array|AddUnique TargetArray (Utilities|Array|Get(acopy) TmpArray _index)))
  (return))